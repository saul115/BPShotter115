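; AI controller for BP_ENEMY1 enemies that drives their behavior and shooting at the player.
; On possess it runs the BP_ENEMIES_TREE behavior tree.
; AI perception updates of the player write the isVisible blackboard key and press or release the enemy's weapon trigger as sight is gained or lost.
; A leftover graph holds an obsolete, disconnected timer and AIMoveTo chase approach that never runs.
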(event OnTargetPerceptionUpdated(AIPerception)
  (params (Actor :type Actor%20Object%20Reference) (Stimulus :type AI%20Stimulus%20Structure))
  (bind _bsuccessfullysensed (Utilities|Struct|BreakAIStimulus Stimulus))
  (Utilities|Casting|CastToBP_Player Actor)
  (AI|Components|Blackboard|SetValueasBool (AI|GetBlackboard 0) (Utilities|Name|MakeLiteralName "isVisible") _bsuccessfullysensed)
  (if _bsuccessfullysensed
    (bind _asbp_enemy1 (Utilities|Casting|CastToBP_ENEMY1 (Pawn|GetControlledPawn)))
    (Default|PressTrigger (Variables|/Game/Blueprints/Enemies/Pawns/BP_ENEMY1.BP_ENEMY1_C|GetWeapon _asbp_enemy1))
    (else
      (bind _asbp_enemy1_2 (Utilities|Casting|CastToBP_ENEMY1 (Pawn|GetControlledPawn)))
      (Default|ReleaseTrigger (Variables|/Game/Blueprints/Enemies/Pawns/BP_ENEMY1.BP_ENEMY1_C|GetWeapon _asbp_enemy1_2)))))

(event EventBeginPlay)

(event EventPossess
  (params (PossessedPawn :type Pawn%20Object%20Reference))
  (Utilities|Casting|CastToBP_ENEMY1 PossessedPawn)
  (AI|RunBehaviorTree "/Game/Blueprints/Enemies/AI/BP_ENEMIES_TREE.BP_ENEMIES_TREE"))

(fn ConstructionScript)

(event Custom|SearchToPlayer)