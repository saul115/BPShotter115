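; BP_ENEMY2 is an enemy Blueprint that carries a weapon and tracks its own health and alive state.
; On BeginPlay it spawns a BP_WEAPON1 and snaps it to the hand_rSocket on its mesh.
; Despite their names, CreateHealth subtracts incoming damage from Health, then calls CreateDamage, which sets IsAlive by whether Health remains above zero.
; The file itself neither calls CreateHealth nor reacts to death.
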(event EventBeginPlay
  (bind _returnvalue (Game|SpawnActorfromClass "/Game/Blueprints/Enemies/BP_WEAPON1.BP_WEAPON1_C" (Transformation|GetWorldTransform (Variables|Character|GetMesh)) "AlwaysSpawn" 0 0))
  (Transformation|AttachComponentToComponent _returnvalue (Variables|Character|GetMesh) "hand_rSocket" "SnapToTarget" "SnapToTarget" "SnapToTarget" true))

(fn ConstructionScript)

(fn CreateHealth
  (params (Damage :type Float%20%28single-precision%29))
  (Variables|Default|SetHealth (- (Variables|Default|GetHealth) Damage))
  (CallFunction|CreateDamage))

(fn CreateDamage
  (if (<= (Variables|Default|GetHealth) 0.0)
    (Variables|Default|SetisAlive false)
    (else
      (Variables|Default|SetisAlive true))))