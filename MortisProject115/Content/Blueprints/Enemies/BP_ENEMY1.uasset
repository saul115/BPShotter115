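; BP_ENEMY1 is an enemy that carries a weapon and dies when its health runs out.
; On BeginPlay it spawns a BP_WEAPON1 and snaps it to the hand_rSocket on its mesh.
; PassDamage subtracts incoming damage from Health, updates IsAlive through CalculateDamage, and destroys both the weapon and the enemy once Health reaches zero or below.
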(event EventPassDamage
  (params (doingDamage :type Float%20%28single-precision%29))
  (CallFunction|CalculateHealth doingDamage)
  (if (not (Variables|Default|GetisAlive))
    (Actor|DestroyActor (Variables|Default|GetWeapon))))

(event EventBeginPlay
  (bind _returnvalue (Game|SpawnActorfromClass "/Game/Blueprints/Enemies/BP_WEAPON1.BP_WEAPON1_C" (Transformation|GetWorldTransform (Variables|Character|GetMesh)) "AlwaysSpawn" 0 0))
  (bind _output_get (Variables|Default|SetWeapon _returnvalue))
  (Transformation|AttachComponentToComponent _output_get (Variables|Character|GetMesh) "hand_rSocket" "SnapToTarget" "SnapToTarget" "SnapToTarget" true))

(fn ConstructionScript)

(fn CalculateHealth
  (params (damage :type Float%20%28single-precision%29))
  (Variables|Default|SetHealth (- (Variables|Default|GetHealth) damage))
  (CallFunction|CalculateDamage))

(fn CalculateDamage
  (if (<= (Variables|Default|GetHealth) 0.0)
    (Variables|Default|SetisAlive false)
    (else
      (Variables|Default|SetisAlive true))))